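; Controller for a stalking scene that sequences NPC dialogue and crowd audio, with hotkeys for a door-smash sound, stopping speech and loading the villa-entrance level.
; Spawn events store criminal and police references and play crowd sound at spawned crowds.
; On BeginPlay, scene 3.2 plays a criminal line, then randomly branches into a solo or police-criminal follow-up.
; PlaySpeechLoop feeds scene/line parameters to a SoundCue and polls until playback ends.
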(event Custom|Spawned_Criminal
  (params (SpawnedCriminal :type BP%20Criminal%20Object%20Reference))
  ;[0 1 0.01562] 스폰 이벤트
  (Variables|Default|SetCriminalRef SpawnedCriminal))

(event Custom|Spawned_Crowd
  (params (SpawnedCrowd :type BP%20Crowd%20Object%20Reference))
  (bind _returnvalue (Transformation|GetActorLocation SpawnedCrowd))
  ;[0 1 0.01562] 스폰 이벤트
  (Audio|PlaySoundatLocation "/Game/Sounds/01_Stalking/av_Crowd.av_Crowd" (Math|Vector|MakeVector (.x _returnvalue) (.y _returnvalue) (+ (.z _returnvalue) 123.0)) "0, 0, 0" 1.0 1.0 0.0 0 0 0 0))

(event Custom|Spawned_Police
  (params (SpawnedPolice :type BP%20Police%20Object%20Reference))
  ;[0 1 0.01562] 스폰 이벤트
  (if (Utilities|ClassIsChildOf (Utilities|GetClass SpawnedPolice) "/Game/MetaHumans/Geonwoo/BP_Geonwoo.BP_Geonwoo_C")
    (Variables|Default|SetPoliceARef SpawnedPolice)
    (else
      (Variables|Default|SetPoliceBRef SpawnedPolice))))

(event Custom|StopPlaySpeechLoop
  (Utilities|PlaySpeechLoop (Variables|Default|GetCriminalRef) 1) ; enters at StopButton
)

(event EventBeginPlay
  (Utilities|FlowControl|Delay 0.1)
  (switch name (Variables|Default|GetSceneNum)
    (:3.2
      (Utilities|PlaySpeechLoop (Variables|Default|GetCriminalRef) 1)
      ;[0 0.9766 1] 3-2-1 or 3-2-2
      (if (Math|Random|RandomBool)
        (Utilities|PlaySpeechLoop (Variables|Default|GetCriminalRef) 1 2)
        (else
          (Utilities|PlaySpeechLoop (Variables|Default|GetPoliceARef) 1 3)
          (Utilities|PlaySpeechLoop (Variables|Default|GetCriminalRef) 1 4))))))

(event Input|KeyboardEvents|1
  (params (Key :type Key%20Structure :default "None"))
  (:Pressed
    (Audio|PlaySoundatLocation "/Game/Sounds/Ambience/Smash/as_ch_DoorSmash.as_ch_DoorSmash" (Transformation|GetActorLocation (Variables|Default|GetCriminalRef)) "0, 0, 0" 1.0 1.0 0.0 0 0 0 0)))

(event Input|KeyboardEvents|2
  (params (Key :type Key%20Structure :default "None"))
  (:Pressed
    (Utilities|StopSpeech)))

(event Input|KeyboardEvents|SpaceBar
  (params (Key :type Key%20Structure :default "None"))
  (:Pressed
    (Game|OpenLevel(byName) "S3-1_Stalking_VillaEntrance")))

(fn ConstructionScript)