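; BP_MainCharacter is an NPC character Blueprint with debug reactions to three emotions: Anger, Joy and Sad.
; Each emotion has a custom event that calls a matching function, which prints the passed key with the emotion name.
; An unconnected chain casts player pawn 0 to VR_Pawn and binds these events to its Anger, Joy and Sad dispatchers.
; BeginPlay is empty, so that binding never runs.
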(event Custom|DspAngerEvent
  (params (WhatKey :type Integer))
  (CallFunction|Anger WhatKey))

(event Custom|DspJoyEvent
  (params (WhatKey :type Integer))
  (CallFunction|Joy WhatKey))

(event Custom|DspSadEvent
  (params (WhatKey :type Integer))
  (CallFunction|Sad WhatKey))

(event EventBeginPlay)

(event Collision|EventActorBeginOverlap
  (params (OtherActor :type Actor%20Object%20Reference)))

(event EventTick
  (params (DeltaSeconds :type Float%20%28single-precision%29)))

(fn ConstructionScript)

(fn Anger
  (params (WhatKey :type Integer))
  (Development|PrintText (Utilities|Text|FormatText "{WhatKey}: Anger" WhatKey)))

(fn Joy
  (params (WhatKey :type Integer))
  (Development|PrintText (Utilities|Text|FormatText "{WhatKey}: Joy" WhatKey)))

(fn Sad
  (params (WhatKey :type Integer))
  (Development|PrintText (Utilities|Text|FormatText "{WhatKey}: Sad" WhatKey)))