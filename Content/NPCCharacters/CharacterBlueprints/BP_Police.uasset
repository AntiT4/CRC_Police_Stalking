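; BP_Police is a police NPC character Blueprint that inherits its behavior from a parent class.
; It overrides the Anger, Joy and Sad emotion functions, each passing WhatKey to the parent version and then printing a "_Police" debug tag.
; BeginPlay and the construction script only call their parents, while the overlap and Tick events are unused placeholders.
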(event EventBeginPlay
  (|CallParentFunction))

(event Collision|EventActorBeginOverlap
  (params (OtherActor :type Actor%20Object%20Reference)))

(event EventTick
  (params (DeltaSeconds :type Float%20%28single-precision%29)))

(fn ConstructionScript
  (|CallParentFunction))

(fn Anger
  (params (WhatKey :type Integer))
  (|CallParentFunction WhatKey)
  (Development|PrintText "_Police"))

(fn Joy
  (params (WhatKey :type Integer))
  (|CallParentFunction WhatKey)
  (Development|PrintText "_Police"))

(fn Sad
  (params (WhatKey :type Integer))
  (|CallParentFunction WhatKey)
  (Development|PrintText "_Police"))