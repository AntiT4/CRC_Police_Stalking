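; BP_Interact is an interactable actor that can be hovered and selected with the left trigger input.
; BeginHover and EndHover toggle IsHoverd and switch the static mesh's custom depth stencil value, likely for a highlight effect.
; TriggerLeft sets IsSelected and prints a debug message without checking hover, as the IsHoverd check runs only on BeginPlay before the same selection logic.
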(event EventBeginPlay
  (if (Variables|Default|GetIsHoverd)
    (Variables|Default|SetIsSelected true)
    (Development|PrintText "selected actor" true true "(R=0.000000,G=0.000000,B=0.000000,A=1.000000)" 1e+01)))

(event Collision|EventActorBeginOverlap
  (params (OtherActor :type Actor%20Object%20Reference)))

(event EventTick
  (params (DeltaSeconds :type Float%20%28single-precision%29)))

(event Input|ActionEvents|InputActionTriggerLeft
  (params (Key :type Key%20Structure :default "None"))
  (:Pressed
    (Variables|Default|SetIsSelected true)
    (Development|PrintText "selected actor" true true "(R=0.000000,G=0.000000,B=0.000000,A=1.000000)" 1e+01)))

(fn ConstructionScript)

(fn BeginHover
  (Rendering|SetCustomDepthStencilValue (Variables|Default|GetStaticMesh) 1)
  (Variables|Default|SetIsHoverd true))

(fn EndHover
  (Rendering|SetCustomDepthStencilValue (Variables|Default|GetStaticMesh) 0)
  (Variables|Default|SetIsHoverd false))